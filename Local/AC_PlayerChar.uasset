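; Player character component for a Conan Exiles clan-control mod that enforces guild rank rules on building, placeable and thrall placement.
; The server sends the player's rank settings and clan base cylinder to the client, which requests updates on guild, rank or settings changes.
; Client Tick watches the build and thrall systems, cancelling forbidden placements with a HUD notice.
; Respawn placeables are exempt, and a global option blocks solo players from building.
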(event `self.ReceiveBeginPlay`
  (`parent.ReceiveBeginPlay`))

(event `self.PreInitialize`
  (if (not (`KismetSystemLibrary.IsServer`))
    (`/Engine/EditorBlueprintResources/StandardMacros.DoOnce` false
      (:`Completed`
        (bind _ascharacter (cast `Character` (`self.GetOwner`)))
        (if (== _ascharacter (`GameplayStatics.GetPlayerCharacter` 0))
          (`self.ServerRequestUpdateDirective`)
          (else
            (`self.SetComponentTickEnabled` false) ; On Clients disable Tick of other player scopes
          ))))))

(event `self.PostInitialize`
  (`parent.PostInitialize`)
  (if (`KismetSystemLibrary.IsServer`)
    (add `/Game/Mods/ControlClan/MC_ControlClan.ServerSettingsUpdated` (`self.mc`) (delegate `ServerSettingsUpdated`))
    (set `self.initializedPostServer` true)))

(event `ServerSettingsUpdated`
  (params (guild :type String))
  (if (`KismetStringLibrary.EqualEqual_StrStr` guild (`self.guildName`))
    (`self.ClientSettingHasBeenUpdated`)))

(event `ClientSettingHasBeenUpdated`
  (`self.ServerRequestUpdateDirective`)
  (bind _asconan_character (cast `ConanCharacter` (`GameplayStatics.GetPlayerCharacter` 0)))
  (`ConanCharacter.ClientHUDShowFIFOAtLocation` _asconan_character "The guildmaster has changed the rank settings." "Low"))

(event `/Game/Mods/ControlClan/ClanMemberMonitoringInterface.StartMonitoring`
  (`self.MessageLog` "Event Start Monitoring" (`self.DebugLevel`)
    (:`Output`
      (set `self.initializedPostClient` true))))

(event `self.ReceiveTick`
  (params (DeltaSeconds :type "Float (single-precision)"))
  (bind _returnvalue (`self.hasBase`))
  (bind _returnvalue_2 (`self.hasBase`))
  (bind _clientthrallsystem (`self.clientThrallSystem`))
  (bind _clientbuildsystemv2 (`self.clientBuildSystemV2`))
  (bind _clientbuildsystemv2_2 (`self.clientBuildSystemV2`))
  (bind _initializedpostserver (`self.initializedPostServer`))
  (bind _initialized (`self.initialized`))
  (bind _returnvalue_3 (and _initializedpostserver (`KismetSystemLibrary.IsServer`)))
  (bind _isbuilding (`BuildSystemComponent.IsBuilding` _clientbuildsystemv2))
  (bind _globalguildenforcer (`/Game/Mods/ControlClan/MC_ControlClan.GlobalGuildEnforcer` (`self.mc`)))
  (bind _buildingbrushplaceable (`/Game/Systems/Building/BP_BuildSystem_v2.BuildingBrushPlaceable` (`self.clientBuildSystemV2`)))
  (bind _returnvalue_4 (and (`self.initializedPostClient`) (not _initializedpostserver)))
  (bind _returnvalue_5 (and (not (`self.InGuild`)) _globalguildenforcer))
  (`parent.ReceiveTick` DeltaSeconds)
  (if (`self.initialized`)
    (if (`self.initializedAll`)
      (if (not (`KismetSystemLibrary.IsServer`))
        (if (`self.hasBase`)
          (bind _isplayerinsidebase (`self.isPlayerInBase`))
          (if (!= _isplayerinsidebase (`self.playerInsideBase`))
            (if (`self.baseBorderLogEnabled`)
              (bind _asconan_character (cast `ConanCharacter` (`GameplayStatics.GetPlayerCharacter` 0))
                (:`then`
                  (`ConanCharacter.ClientHUDShowFIFOAtLocation` _asconan_character (select `bool` _isplayerinsidebase :`false` "You left the clan base." :`true` "You entered the clan base." :!type "Text") "Low"))
                (:`CastFailed`
                  _)))
            (bind _output_get (set `/Game/Mods/ControlClan/MC_ControlClan.playerInsideBase` _isplayerinsidebase (`self.mc`)))
            (set `self.playerInsideBase` _output_get)))
        (`|ExecutionSequence`
          (:`then_0`
            (bind _asbase_player_char (cast `/Game/Characters/BasePlayerChar` (`GameplayStatics.GetPlayerCharacter` 0)))
            (bind _returnvalue_6 (`ConanCharacter.GetGuild` _asbase_player_char))
            (`/Engine/EditorBlueprintResources/StandardMacros.IsValid` _returnvalue_6
              (:`Is Valid`
                (if (`KismetStringLibrary.NotEqual_StrStr` (`/Game/Mods/ControlClan/MC_ControlClan.playerGuildName` (`self.mc`)) (`Guild.GetGuildName` _returnvalue_6))
                  (`self.ServerRequestUpdateDirective` :!label _label)
                  (else
                    (for _array_element (`Guild.GetGuildMembers` _returnvalue_6)
                      (bind (_charactername _playernickname _playernetid _level _isonline _rank) (break `PlayerInfo` _array_element))
                      (`/Game/Systems/BP_MacroGlobal.And+Branch` (`KismetStringLibrary.EqualEqual_StrStr` _charactername (`ConanCharacter.GetCharacterName` _asbase_player_char)) (`|EnumInequality` _rank (`self.rank`))
                        (:`True`
                          (goto _label)))))))
              (:`Is Not Valid`
                (if (`/Game/Mods/ControlClan/MC_ControlClan.playerCharacterInGuild` (`self.mc`))
                  (goto _label)))))
          (:`then_1`
            (if (`self.updatePending`)
              (set `self.updatePending` false)
              (`|ExecutionSequence`
                (:`then_0`
                  (set `self.placingRestrictedForBuilding` false)
                  (`self.isPlacingRestricted` "NewEnumerator0"
                    (:`OutputPin`
                      (set `self.placingRestrictedForBuilding` true))))
                (:`then_1`
                  (set `self.placingRestrictedForPlacable` false)
                  (`self.isPlacingRestricted` "NewEnumerator1"
                    (:`OutputPin`
                      (set `self.placingRestrictedForPlacable` true))))
                (:`then_2`
                  (set `self.placingRestrictedForThrall` false)
                  (`self.isPlacingRestricted` "NewEnumerator2"
                    (:`OutputPin`
                      (set `self.placingRestrictedForThrall` true))))
                (:`then_3`
                  (bind _charactername_2 (`self.characterName`)
                    (:`then`
                      (`self.MessageLog` (`KismetStringLibrary.Concat_StrStr` "Update processed,\nMonitor Build/Place/Thrall: " (`KismetStringLibrary.Conv_BoolToString` (`self.placingRestrictedForBuilding`)) "," (`KismetStringLibrary.Conv_BoolToString` (`self.placingRestrictedForPlacable`)) "," (`KismetStringLibrary.Conv_BoolToString` (`self.placingRestrictedForThrall`))) "INFOL_IMPORTANT"
                        (:`Output`
                          (`self.MessageLog` (`KismetStringLibrary.Concat_StrStr` "updated for: " (`KismetStringLibrary.Conv_BoolToString` (`self.InGuild`)) "," (`|GetEnumeratorNameAsString` (`self.rank`)) "," (`self.guildName`) "   --- " _charactername_2) "INFOL_IMPORTANT")))))))))
          (:`then_2`
            (`/Engine/EditorBlueprintResources/StandardMacros.IsValid` _clientbuildsystemv2_2
              (:`Is Valid`
                (if (`BuildSystemComponent.IsBuilding` _clientbuildsystemv2_2)
                  (`/Engine/EditorBlueprintResources/StandardMacros.IsValid` _buildingbrushplaceable
                    (:`Is Valid`
                      (if (not (`KismetSystemLibrary.DoesImplementInterface` _buildingbrushplaceable "/Game/Systems/Building/Placeables/PlaceableRespawnPointInterface.PlaceableRespawnPointInterface_C"))
                        (`|ExecutionSequence` :!label _label_2
                          (:`then_0`
                            (if (or _returnvalue_5 (`self.placingRestrictedForBuilding`) _returnvalue_2)
                              (`/Engine/EditorBlueprintResources/StandardMacros.IsValid` _clientbuildsystemv2
                                (:`Is Valid`
                                  (if (and _isbuilding (not (`/Game/Systems/Building/BP_BuildSystem_v2.IsBuildingPlaceables` _clientbuildsystemv2)))
                                    (if (`/Game/Mods/ControlClan/MC_ControlClan.playerCharacterInGuild` (`self.mc`))
                                      (bind _access (`self.hasAccess` "NewEnumerator0"))
                                      (if _access
                                        (if _returnvalue_2 :!label _label_3
                                          (if (`self.detailTracking`)
                                            (bind _location (`/Game/Systems/Building/BP_BuildSystem_v2.GetBuildingBrushLocation` _clientbuildsystemv2))
                                            (bind _returnvalue_7 (`self.isInsideCylinder` _location (`self.baseXYRadius`)))
                                            (if _returnvalue_7
                                              (`BuildSystemComponent.StopBuilding` _clientbuildsystemv2 :!label _label_4)
                                              (bind _asconan_character_2 (cast `ConanCharacter` (`GameplayStatics.GetPlayerCharacter` 0)))
                                              (`ConanCharacter.ClientHUDShowFIFOAtLocation` _asconan_character_2 (select `bool` _returnvalue_5 :`false` "Codex: \nThe guildmaster has not allowed you to build here." :`true` "Server Rule: \nBuildings for solo players forbidden.\nYou must create or join a guild.") "Low")
                                              (bind _foundwidgets (`WidgetBlueprintLibrary.GetAllWidgetsOfClass` "/Script/ConanSandbox.ShortcutBarBase"))
                                              (if (> (`KismetArrayLibrary.Array_Length` _foundwidgets) 0)
                                                (bind _asw_shortcut_bar (cast `/Game/UI/HUD/W_ShortcutBar` (`KismetArrayLibrary.Array_Get` _foundwidgets)))
                                                (`Widget.SetVisibility` (`/Game/UI/HUD/W_ShortcutIcon.IsActiveView` (`/Game/UI/HUD/W_ShortcutBar.Slot0` _asw_shortcut_bar)) "Hidden")
                                                (`Widget.SetVisibility` (`/Game/UI/HUD/W_ShortcutIcon.IsActiveView` (`/Game/UI/HUD/W_ShortcutBar.Slot1` _asw_shortcut_bar)) "Hidden")
                                                (`Widget.SetVisibility` (`/Game/UI/HUD/W_ShortcutIcon.IsActiveView` (`/Game/UI/HUD/W_ShortcutBar.Slot2` _asw_shortcut_bar)) "Hidden")
                                                (`Widget.SetVisibility` (`/Game/UI/HUD/W_ShortcutIcon.IsActiveView` (`/Game/UI/HUD/W_ShortcutBar.Slot3` _asw_shortcut_bar)) "Hidden")
                                                (`Widget.SetVisibility` (`/Game/UI/HUD/W_ShortcutIcon.IsActiveView` (`/Game/UI/HUD/W_ShortcutBar.Slot4` _asw_shortcut_bar)) "Hidden")
                                                (`Widget.SetVisibility` (`/Game/UI/HUD/W_ShortcutIcon.IsActiveView` (`/Game/UI/HUD/W_ShortcutBar.Slot5` _asw_shortcut_bar)) "Hidden")
                                                (`Widget.SetVisibility` (`/Game/UI/HUD/W_ShortcutIcon.IsActiveView` (`/Game/UI/HUD/W_ShortcutBar.Slot6` _asw_shortcut_bar)) "Hidden")
                                                (`Widget.SetVisibility` (`/Game/UI/HUD/W_ShortcutIcon.IsActiveView` (`/Game/UI/HUD/W_ShortcutBar.Slot7` _asw_shortcut_bar)) "Hidden"))
                                              (else
                                                (`self.MessageLog` "is outside" "INFOL_IMPORTANT"))))
                                          (else
                                            (goto _label_4)))
                                        (else
                                          (goto _label_4)))
                                      (elif _globalguildenforcer
                                        (goto _label_4))))))))
                          (:`then_1`
                            (if (or _returnvalue_2 (`self.placingRestrictedForPlacable`))
                              (`/Engine/EditorBlueprintResources/StandardMacros.IsValid` _clientbuildsystemv2
                                (:`Is Valid`
                                  (if (and _isbuilding (`/Game/Systems/Building/BP_BuildSystem_v2.IsBuildingPlaceables` _clientbuildsystemv2))
                                    (bind _access_2 (`self.hasAccess` "NewEnumerator1"))
                                    (if _access_2
                                      (goto _label_3)
                                      (else
                                        (goto _label_4)))))))))))
                    (:`Is Not Valid`
                      (goto _label_2)))))))
          (:`then_3`
            (if (or _returnvalue (`self.placingRestrictedForThrall`))
              (`/Engine/EditorBlueprintResources/StandardMacros.IsValid` _clientthrallsystem
                (:`Is Valid`
                  (if (`ThrallSystemComponent.IsPlacingThrall` _clientthrallsystem)
                    (bind _access_3 (`self.hasAccess` "NewEnumerator2"))
                    (if _access_3
                      (if _returnvalue
                        (if (`self.detailTracking`)
                          (bind _returnvalue_8 (`self.isInsideCylinder` (`Actor.K2_GetActorLocation` (`/Game/Systems/Thrall/BP_ThrallSystemComponent.BrushActor` _clientthrallsystem)) (`self.baseXYRadius`)))
                          (if _returnvalue_8
                            (`ThrallSystemComponent.StopPlacingThrall` _clientthrallsystem (`/Game/Systems/Thrall/BP_ThrallSystemComponent.SourceThrallItem` _clientthrallsystem) :!label _label_5)
                            (bind _asconan_character_3 (cast `ConanCharacter` (`GameplayStatics.GetPlayerCharacter` 0)))
                            (`ConanCharacter.ClientHUDShowFIFOAtLocation` _asconan_character_3 "Codex: The guildmaster has not allowed you to place here." "Low")
                            (else
                              (`self.MessageLog` "is outside" "INFOL_INFO0"))))
                        (else
                          (goto _label_5)))
                      (else
                        (goto _label_5))))))))))
      (elif (and (or _returnvalue_4 _returnvalue_3) _initialized)
        (set `self.initializedAll` true)
        (else
          (`self.MessageLog` (`KismetStringLibrary.Concat_StrStr` "init pending. status: " (`KismetStringLibrary.Conv_BoolToString` _initialized) " " (`KismetStringLibrary.Conv_BoolToString` _returnvalue_4) " / " (`KismetStringLibrary.Conv_BoolToString` _returnvalue_3)) "INFOL_IMPORTANT"))))))

(event `ServerRequestUpdateDirective`
  (bind _mc (`self.mc`))
  (`self.MessageLog` "ServerRequestUpdateDirective" (`self.DebugLevel`)
    (:`Output`
      (set `self.baseXYRadius` (0.0 0.0 0.0))
      (`self.ClientClearDirectives`)
      (bind _asbase_player_char (cast `/Game/Characters/BasePlayerChar` (`self.GetOwner`)))
      (bind _returnvalue (`ConanCharacter.GetGuild` _asbase_player_char))
      (bind _output_get (set `/Game/Mods/ControlClan/MC_ControlClan.playerCharacterInGuild` (`KismetSystemLibrary.IsValid` _returnvalue) _mc))
      (bind _output_get_2 (set `self.InGuild` _output_get))
      (if _output_get_2
        (set `self.guildName` (`Guild.GetGuildName` _returnvalue))
        (for _array_element (`Guild.GetGuildMembers` _returnvalue)
          (bind (_charactername _playernickname _playernetid _level _isonline _rank) (break `PlayerInfo` _array_element))
          (if (`KismetStringLibrary.EqualEqual_StrStr` (`ConanCharacter.GetCharacterName` _asbase_player_char) _charactername)
            (bind _output_get_3 (set `self.rank` _rank))
            (for _array_element_2 (`/Game/Mods/ControlClan/MC_ControlClan.settings` _mc)
              (bind _returnvalue_2 (`Guild.GetGuildName` _returnvalue))
              (bind (_guildname _rank_2) (break `/Game/Mods/ControlClan/Struct_RankTargetSetting` _array_element_2))
              (`/Game/Systems/BP_MacroGlobal.And+Branch` (`KismetStringLibrary.EqualEqual_StrStr` _returnvalue_2 _guildname) (`|EnumEquality` _output_get_3 _rank_2)
                (:`True`
                  (`self.ClientUpdateDirective` _array_element_2))))))
        (for _array_element_3 (`/Game/Mods/ControlClan/MC_ControlClan.baseSetting` _mc)
          (bind (_guildname_2 _xyradius) (break `/Game/Mods/ControlClan/Struct_ClanBaseSetting` _array_element_3))
          (if (`KismetStringLibrary.EqualEqual_StrStr` _returnvalue_2 _guildname_2)
            (set `self.baseXYRadius` _xyradius)))
        (else
          (set `self.guildName` "")))
      (`self.MessageLog` (`KismetStringLibrary.Concat_StrStr` "ServerUpdate on ClientUpdateDirectiveFinished: " (`KismetStringLibrary.Conv_BoolToString` (`self.InGuild`)) " " (`|GetEnumeratorNameAsString` (`self.rank`)) " " (`self.guildName`) ", XYRadius = " (`KismetStringLibrary.Conv_VectorToString` (`self.baseXYRadius`))) "INFOL_IMPORTANT"
        (:`Output`
          (`self.ClientUpdateDirectivesFinished` (`self.InGuild`) (`self.rank`) (`self.guildName`) (`self.baseXYRadius`)))))))

(event `ClientClearDirectives`
  (`KismetArrayLibrary.Array_Clear` (`/Game/Mods/ControlClan/MC_ControlClan.playerRankSettingArray` (`self.mc`)))
  (`self.MessageLog` "----- DIRECTIVES ----" (enumliteral `EDebugLevel` "INFOL_IMPORTANT")))

(event `ClientUpdateDirective`
  (params (setting :type "/Game/Mods/ControlClan/Struct_RankTargetSetting Structure"))
  (bind (_guildname _rank _target _level) (break `/Game/Mods/ControlClan/Struct_RankTargetSetting` setting))
  (`KismetArrayLibrary.Array_Add` (`/Game/Mods/ControlClan/MC_ControlClan.playerRankSettingArray` (`self.mc`)) setting)
  (`self.MessageLog` (`KismetStringLibrary.Concat_StrStr` _guildname ": " (`|GetEnumeratorNameAsString` _rank) "/" (`|GetEnumeratorNameAsString` _target) " := " (`|GetEnumeratorNameAsString` _level)) (enumliteral `EDebugLevel` "INFOL_IMPORTANT")))

(event `ClientUpdateDirectivesFinished`
  (params (InGuild :type Boolean) (rank :type "ERank Enum") (guildName :type String) (baseXYRadius :type "Vector Structure"))
  (bind _output_get (set `self.InGuild` InGuild))
  (bind _output_get_2 (set `self.rank` rank))
  (bind _output_get_3 (set `self.guildName` guildName))
  (bind _output_get_4 (set `self.baseXYRadius` baseXYRadius))
  (`/Game/Mods/ControlClan/MC_ControlClan.ClientDirectivesUpdated` (`self.mc`) _output_get _output_get_2 _output_get_3 _output_get_4)
  (`self.MessageLog` "----- ------------- ----" (enumliteral `EDebugLevel` "INFOL_IMPORTANT")))

(event `SetVisualizeBase`
  (params (visible :type Boolean))
  (bind _basexyradius (`self.baseXYRadius`))
  (bind _x (.x _basexyradius))
  (bind _y (.y _basexyradius))
  (set `self.baseBorderLogEnabled` visible)
  (`self.MessageLog` (`KismetStringLibrary.Concat_StrStr` "--- BASE VISIBILITY ---> " (`KismetStringLibrary.Conv_BoolToString` visible) " " (`KismetStringLibrary.Conv_VectorToString` _basexyradius)) "INFOL_INFO2"
    (:`Output`
      (`KismetSystemLibrary.DrawDebugCylinder` (`KismetMathLibrary.MakeVector` _x _y -40000.0) (`KismetMathLibrary.MakeVector` _x _y 40000.0) (.z _basexyradius) 12 (struct :`R` 1.0 :`B` 0.147743 :`A` 0.25) 20.0 5.0)
      (bind _asconan_character (cast `ConanCharacter` (`GameplayStatics.GetPlayerCharacter` 0)))
      (`ConanCharacter.ClientHUDShowFIFOAtLocation` _asconan_character "clan base border debug switched" "Low"))))

(fn `checkInitialized`
  (returns (isInitialized :type Boolean))
  (if (`/Game/Mods/ControlClan/MC_ControlClan.preinitialized` (`self.mc`))
    (bind _charactername (`self.characterName`)
      (:`then`
        (if (> (`KismetStringLibrary.Len` _charactername) 0)
          (`self.initializeMonitor`)
          (`self.MessageLog` "Check initialized succeeded." "INFOL_IMPORTANT"
            (:`Output`
              (return true)))
          (else
            _)))
      (:`CastFailed`
        (`self.MessageLog` "waiting (Check initialized)... bpc cast failed" "INFOL_CODEERROR"
          (:`Output`
            _))))
    (else
      (`self.MessageLog` "waiting (Check initialized) not preinitialized ..." "INFOL_IMPORTANT"
        (:`Output`
          _))))
  (return false))

(fn `GetTargetLevel`
  (params (target :type "/Game/Mods/ControlClan/ESettingTarget Enum"))
  (returns (level :type "/Game/Mods/ControlClan/ESettingLevel Enum"))
  (for _array_element (`/Game/Mods/ControlClan/MC_ControlClan.playerRankSettingArray` (`self.mc`))
    (bind (_guildname _rank _target _level) (break `/Game/Mods/ControlClan/Struct_RankTargetSetting` _array_element))
    (`/Game/Systems/BP_MacroGlobal.And+Branch` (`|EnumEquality` _rank (`self.rank`)) (`|EnumEquality` _target target)
      (:`True`
        (return _level))))
  (return (select `ERank` (`self.rank`) :`Recruit` "NewEnumerator0" :`Member` "NewEnumerator0" :`Officer` "NewEnumerator3" :`GuildMaster` "NewEnumerator4" :`ERank_MAX` "NewEnumerator4" :!type "/Game/Mods/ControlClan/ESettingLevel Enum")))