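; Actor component for thrall NPCs that toggles whether they can be interacted with, based on an inherited access check.
; On tick, once initialized and when an update is pending or a border is passed, it sets the owner capsule's response on a custom trace channel to Overlap or Ignore.
; The first such pass disables ticking for non-thrall NPCs.
; It also overrides parent helpers for naming and initialization, and logs with a ControlClan prefix.
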(event `self.ReceiveBeginPlay`
  (`parent.ReceiveBeginPlay`))

(event `self.ReceiveTick`
  (params (DeltaSeconds :type "Float (single-precision)"))
  (bind _currentresponse (`self.CurrentResponse`))
  (`parent.ReceiveTick` DeltaSeconds)
  (if (and (`self.initialized`) (or (`self.updatePending`) (`self.baseBorderPassed`)))
    (set `self.updatePending` false)
    (if (`self.initializedThrallCheck`)
      (bind _access (`self.hasAccess` "NewEnumerator2" :!label _label))
      (bind _returnvalue (select `bool` _access :`false` "ECR_Ignore" :`true` "ECR_Overlap" :!type "ECollisionResponse Enum"))
      (if (`|EnumInequality` (`self.currentResponse`) _returnvalue)
        (set `self.currentResponse` _returnvalue)
        (bind _asbase_npc (cast `/Game/Characters/BaseNPC` (`self.GetOwner`)))
        (`PrimitiveComponent.SetCollisionResponseToChannel` (`Character.CapsuleComponent` _asbase_npc) "ECC_GameTraceChannel16" _currentresponse)
        (`self.MessageLog` (`KismetStringLibrary.Concat_StrStr` "interact changed to " (`|GetEnumeratorNameAsString` _currentresponse)) (`self.DebugLevel`)))
      (else
        (set `self.initializedThrallCheck` true)
        (bind _asbase_npc_2 (cast `/Game/Characters/BaseNPC` (`self.GetOwner`))
          (:`then`
            (if (`ConanCharacter.IsNonThrallNPC` _asbase_npc_2)
              (`self.SetComponentTickEnabled` self false)
              (`self.MessageLog` "stop monitoring." (`self.DebugLevel`))
              (else
                (goto _label))))
          (:`CastFailed`
            (`self.MessageLog` "cast failed" "INFOL_CODEERROR")))))))

(fn `checkInitialized`
  (returns (isInitialized :type Boolean))
  (return true))

(fn `getOwnerName`
  (returns (name :type String))
  (bind _name (`parent.getOwnerName`))
  (return _name))

(fn `targetPrefixName`
  (returns (NewParam :type String))
  (bind _asbase_npc (cast `/Game/Characters/BaseNPC` (`self.GetOwner`))
    (:`then`
      (return (`ConanCharacter.GetCharacterName` _asbase_npc)))
    (:`CastFailed`
      (return "-"))))