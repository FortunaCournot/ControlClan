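; Building access component that toggles whether the owning BP_BuildingBase responds to a custom interaction channel, based on access rights.
; When initialized, Tick waits for a pending update or base border crossing, then sets the instanced mesh's channel response to Overlap or Ignore, only on change.
; The initialization check requires mesh instances and disables ticking for brushes.
; It extends a parent component and prefixes debug logs with the controlling clan.
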(event `self.ReceiveBeginPlay`
  (`parent.ReceiveBeginPlay`))

(event `self.ReceiveTick`
  (params (DeltaSeconds :type "Float (single-precision)"))
  (bind _currentresponse (`self.CurrentResponse`))
  (`parent.ReceiveTick` DeltaSeconds)
  (if (and (`self.initialized`) (or (`self.updatePending`) (`self.baseBorderPassed`)))
    (set `self.updatePending` false)
    (bind _access (`self.hasAccess` "NewEnumerator0"))
    (bind _returnvalue (select `bool` _access :`false` "ECR_Ignore" :`true` "ECR_Overlap" :!type "ECollisionResponse Enum"))
    (if (`|EnumInequality` (`self.currentResponse`) _returnvalue)
      (set `self.currentResponse` _returnvalue)
      (bind _asbp_building_base (cast `/Game/Systems/Building/BP_BuildingBase` (`self.GetOwner`))
        (:`then`
          (`PrimitiveComponent.SetCollisionResponseToChannel` (`BuildingBase.InstancedBuildingMesh` _asbp_building_base) "ECC_GameTraceChannel16" _currentresponse)
          (`self.MessageLog` (`KismetStringLibrary.Concat_StrStr` "interact changed to " (`|GetEnumeratorNameAsString` _currentresponse)) (`self.DebugLevel`)))
        (:`CastFailed`
          (`self.MessageLog` "not a buildingbase" "INFOL_CODEERROR"
            (:`Output`
              (set `self.updatePending` false))))))))

(fn `checkInitialized`
  (returns (isInitialized :type Boolean))
  (bind _asbp_building_base (cast `/Game/Systems/Building/BP_BuildingBase` (`self.GetOwner`))
    (:`then`
      (if (`BuildableBase.IsABrush` _asbp_building_base)
        (`self.SetComponentTickEnabled` false)
        (else
          (return (> (`InstancedStaticMeshComponent.GetInstanceCount` (`BuildingBase.InstancedBuildingMesh` _asbp_building_base)) 0)))))
    (:`CastFailed`
      _))
  (return false))