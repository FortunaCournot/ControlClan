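; Base component for ControlClan permission targets, deciding whether the player may access a given target type.
; Tick finds MC_ControlClan, waits for initialization, binds directive updates to flag UpdatePending, then tracks base border crossings.
; HasAccess combines the target's permission level with a cylinder inside-base test, letting [character], [guild] or [public] name prefixes override interact denials.
; Init hooks and name getters are stubs, apparently for subclasses.
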(event `self.ReceiveBeginPlay`)

(event `self.ReceiveTick`
  (params (DeltaSeconds :type "Float (single-precision)"))
  (bind _playerinsidebase (`/Game/Mods/ControlClan/MC_ControlClan.playerInsideBase` (`self.mc`)))
  (if (`self.initialized`)
    (if (!= _playerinsidebase (`self.playerInsideBase`))
      (set `self.playerInsideBase` _playerinsidebase)
      (set `self.baseBorderPassed` true)
      (else
        (set `self.baseBorderPassed` false)))
    (else
      (`/Engine/EditorBlueprintResources/StandardMacros.IsValid` (`self.mc`)
        (:`Is Valid`
          (if (`/Game/Mods/ControlClan/MC_ControlClan.initialized` (`self.mc`)) :!label _label
            (bind _isinitialized (`self.checkInitialized`))
            (set `self.DebugLevel` (`/Game/Mods/ControlClan/MC_ControlClan.DebugLevel` (`self.mc`)))
            (set `self.initialized` _isinitialized)
            (`self.PostInitialize`)
            (else
              (`self.PreInitialize`))))
        (:`Is Not Valid`
          (bind _outactors (`GameplayStatics.GetAllActorsOfClass` "/Game/Mods/ControlClan/MC_ControlClan.MC_ControlClan_C"))
          (if (> (`KismetArrayLibrary.Array_Length` _outactors) 0)
            (set `self.mc` (`KismetArrayLibrary.Array_Get` _outactors))
            (goto _label)))))))

(event `PreInitialize`)

(event `PostInitialize`
  (bind _mc (`self.mc`))
  (`/Engine/EditorBlueprintResources/StandardMacros.IsValid` _mc
    (:`Is Valid`
      (add `/Game/Mods/ControlClan/MC_ControlClan.DirectivesUpdated` _mc (delegate `DirectivesUpdated`))
      (set `self.updatePending` true)
      (set `self.playerInsideBase` (`/Game/Mods/ControlClan/MC_ControlClan.playerInsideBase` (`self.mc`)))
      (set `self.baseBorderPassed` false))
    (:`Is Not Valid`
      (`self.MessageLog` "mc invalid" "INFOL_CODEERROR"))))

(event `DirectivesUpdated`
  (set `self.updatePending` true)
  (`self.MessageLog` "Update Pending! ..." (`self.DebugLevel`)))

(fn `characterPrefixName`
  (returns (prefix :type String))
  (return (`KismetStringLibrary.Concat_StrStr` "[" (`/Game/Mods/ControlClan/MC_ControlClan.playerCharacterName` (`self.mc`)) "]")))

(fn `checkInitialized`
  (returns (isInitialized :type Boolean))
  (`self.MessageLog` "check initialized: true" "INFOL_IMPORTANT"
    (:`Output`
      (return true))))

(fn `getOwnerName`
  (returns (name :type String))
  (return ""))

(fn `guildPrefixName`
  (returns (prefix :type String))
  (return (`KismetStringLibrary.Concat_StrStr` "[" (`/Game/Mods/ControlClan/MC_ControlClan.playerGuildName` (`self.mc`)) "]")))

(fn `hasAccess`
  (params (target :type "/Game/Mods/ControlClan/ESettingTarget Enum"))
  (returns (access :type Boolean))
  (bind _returnvalue (`|GetEnumeratorNameAsString` target))
  (bind _debuglevel (`self.DebugLevel`))
  (bind _mc (`self.mc`))
  (bind _returnvalue_2 (`|GetEnumeratorNameAsString` (`/Game/Mods/ControlClan/MC_ControlClan.playerCharacterGuildRank` _mc)))
  (if (`self.initialized`)
    (bind _value (`/Game/Mods/ControlClan/MC_ControlClan.GetTargetLevel` _mc target))
    (switch `/Game/Mods/ControlClan/ESettingLevel` _value
      (:`NewEnumerator0`
        (if (`self.isInteractTargetClass`)
          ;[1 1 1] OutsideBase
          (set `self.detailTracking` true :!label _label)
          (bind _isplayerinsidebase (`self.isPlayerInBase`))
          (if _isplayerinsidebase
            (bind _returnvalue_3 (`|GetEnumeratorNameAsString` _value))
            (`self.MessageLog` (`KismetStringLibrary.Concat_StrStr` _returnvalue_2 " access to " _returnvalue ": false because level=" _returnvalue_3 "   dt=" (`KismetStringLibrary.Conv_BoolToString` (`self.detailTracking`))) _debuglevel :!label _label_2
              (:`Output`
                ;[1 1 1] Interaction: Object Access override check
                (if (`self.isInteractTargetClass`)
                  (bind _access (`self.hasPrivateOrPublicAccess`))
                  (if _access
                    (return true)
                    (else
                      _)))))
            (else
              (`self.MessageLog` (`KismetStringLibrary.Concat_StrStr` _returnvalue_2 " access to " _returnvalue ": true because level=" _returnvalue_3 "   dt=" (`KismetStringLibrary.Conv_BoolToString` (`self.detailTracking`))) _debuglevel :!label _label_3
                (:`Output`
                  (return true)))))
          (else
            (set `self.detailTracking` true)
            (goto _label_2))))
      (:`NewEnumerator1`
        (if (`self.isInteractTargetClass`)
          (goto _label)
          (else
            (set `self.detailTracking` true :!label _label_4)
            (goto _label_3))))
      (:`NewEnumerator2`
        (if (`self.isInteractTargetClass`)
          (goto _label_4)
          (else
            (goto _label_4))))
      (:`NewEnumerator3`
        (goto _label_4))
      (:`NewEnumerator4`
        (set `self.detailTracking` false)
        (goto _label_3)))
    (return false)
    (else
      (`self.MessageLog` "has access: denied (not initialized)" (`self.DebugLevel`)
        (:`Output`
          (return false))))))

(fn `hasPrivateOrPublicAccess`
  (returns (access :type Boolean))
  (bind _newparam (`self.targetPrefixName`))
  (if (`KismetStringLibrary.StartsWith` _newparam "[")
    (`|ExecutionSequence`
      (:`then_0`
        (bind _prefix (`self.characterPrefixName`))
        (if (`KismetStringLibrary.StartsWith` _newparam _prefix)
          (`self.MessageLog` (`KismetStringLibrary.Concat_StrStr` "access granted to " _newparam) "INFOL_IMPORTANT" :!label _label
            (:`Output`
              (return true)))))
      (:`then_1`
        (bind _prefix_2 (`self.guildPrefixName`))
        (if (`KismetStringLibrary.StartsWith` _newparam _prefix_2)
          (goto _label)))
      (:`then_2`
        (if (`KismetStringLibrary.StartsWith` _newparam "[public]")
          (goto _label)))
      (:`then_3`
        (`self.MessageLog` (`KismetStringLibrary.Concat_StrStr` "access denied to " _newparam) "INFOL_IMPORTANT" :!label _label_2
          (:`Output`
            (return false)))))
    (else
      (goto _label_2))))

(fn `isInsideCylinder`
  (params (actorLocation :type "Vector Structure") (baseXYRadius :type "Vector Structure"))
  (returns (ReturnValue :type Boolean))
  (return (`self.testIsInsideCylinder` actorLocation baseXYRadius)))

(fn `isPlayerInBase`
  (returns (isPlayerInsideBase :type Boolean))
  (bind _playerclanbasexyradius (`/Game/Mods/ControlClan/MC_ControlClan.playerClanBaseXYRadius` (`self.mc`)))
  (if (> (.z _playerclanbasexyradius) 0.0)
    (return (`self.testIsInsideCylinder` (`Actor.K2_GetActorLocation` (`GameplayStatics.GetPlayerCharacter` 0)) _playerclanbasexyradius))
    (else
      (return false))))

(fn `targetPrefixName`
  (returns (NewParam :type String))
  (return "-"))