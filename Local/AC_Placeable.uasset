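; Actor component for placeables that, going by its log tag, is part of a clan-control system, toggling interaction based on access rights.
; On tick, when an update is pending or a base border is passed, it rechecks access and switches the owner's static and skeletal meshes between Overlap and Ignore on a custom trace channel.
; Overrides supply buildable and owner names to the parent, and disable ticking for brushes or non-placeable owners.
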(event `self.ReceiveBeginPlay`
  (`parent.ReceiveBeginPlay`))

(event `self.ReceiveTick`
  (params (DeltaSeconds :type "Float (single-precision)"))
  (bind _debuglevel (`self.DebugLevel`))
  (bind _currentresponse (`self.currentResponse`))
  (bind _returnvalue (`KismetStringLibrary.Concat_StrStr` "interact changed to " (`|GetEnumeratorNameAsString` _currentresponse)))
  (`parent.ReceiveTick` DeltaSeconds)
  (if (and (`self.initialized`) (or (`self.updatePending`) (`self.baseBorderPassed`)))
    (set `self.updatePending` false)
    (bind _access (`self.hasAccess` "NewEnumerator1"))
    (bind _returnvalue_2 (select `bool` _access :`false` "ECR_Ignore" :`true` "ECR_Overlap" :!type "ECollisionResponse Enum"))
    (if (`|EnumInequality` (`self.currentResponse`) _returnvalue_2)
      (set `self.currentResponse` _returnvalue_2)
      (bind _asbp_master_placeables (cast `/Game/Systems/Building/Placeables/BP_Master_Placeables` (`self.GetOwner`)))
      (`|ExecutionSequence`
        (:`then_0`
          (bind _staticmesh (`/Game/Systems/Building/Placeables/BP_Master_Placeables.StaticMesh` _asbp_master_placeables))
          (`/Engine/EditorBlueprintResources/StandardMacros.IsValid` _staticmesh
            (:`Is Valid`
              (`PrimitiveComponent.SetCollisionResponseToChannel` _staticmesh "ECC_GameTraceChannel16" _currentresponse)
              (`self.MessageLog` _returnvalue _debuglevel))))
        (:`then_1`
          (bind _skeletalmesh (`/Game/Systems/Building/Placeables/BP_Master_Placeables.SkeletalMesh` _asbp_master_placeables))
          (`/Engine/EditorBlueprintResources/StandardMacros.IsValid` _skeletalmesh
            (:`Is Valid`
              (`PrimitiveComponent.SetCollisionResponseToChannel` _skeletalmesh "ECC_GameTraceChannel16" _currentresponse)
              (`self.MessageLog` _returnvalue _debuglevel))))))))

(event `self.PostInitialize`
  (`parent.PostInitialize`))

(fn `checkInitialized`
  (returns (isInitialized :type Boolean))
  (bind _asplaceable_base (cast `PlaceableBase` (`self.GetOwner`))
    (:`then`
      (if (`BuildableBase.IsABrush` _asplaceable_base)
        _
        (else
          (return true))))
    (:`CastFailed`
      _))
  (`self.SetComponentTickEnabled` false)
  (return false))

(fn `getOwnerName`
  (returns (name :type String))
  (bind _asplaceable_base (cast `PlaceableBase` (`self.GetOwner`))
    (:`then`
      (bind _returnvalue (`BuildableBase.GetOwnerName` _asplaceable_base))
      (return (`KismetTextLibrary.Conv_TextToString` _returnvalue)))
    (:`CastFailed`
      (return ""))))

(fn `targetPrefixName`
  (returns (NewParam :type String))
  (bind _asplaceable_base (cast `PlaceableBase` (`self.GetOwner`))
    (:`then`
      (return (`KismetTextLibrary.Conv_TextToString` (`BuildableBase.GetBuildableName` _asplaceable_base false))))
    (:`CastFailed`
      (return "-"))))